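; GA_BPTest is a test Gameplay Ability that exercises cost and cooldown commit checks through debug prints in Korean.
; On activation it calls CommitAbility and prints an activation message on success.
; On failure, a sequence checks cost and cooldown separately to report low mana or an active cooldown, then retries the commit with its own success message.
; It applies no other effect and never calls EndAbility.
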(event Ability|EventActivateAbility
  (bind _returnvalue (Ability|CommitAbility))
  (if _returnvalue
    (Development|PrintString "어빌리티 발동")
    (else
      (Utilities|FlowControl|Sequence
        (:then_0
          (bind _returnvalue_2 (Class|GameplayAbility|CheckAbilityCost))
          (if (not _returnvalue_2)
            (Development|PrintString "마나 부족")))
        (:then_1
          (bind _returnvalue_3 (Class|GameplayAbility|CheckAbilityCooldown))
          (if (not _returnvalue_3)
            (Development|PrintString "쿨타임 아직")))
        (:then_2
          (bind _returnvalue_4 (Ability|CommitAbility))
          (if _returnvalue_4
            (Development|PrintString "Test 어빌리티 발동")))))))

(event Ability|EventOnEndAbility
  (params (bWasCancelled :type Boolean)))